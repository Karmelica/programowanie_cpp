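; AI controller for enemy characters that switches them between patrol and combat based on perception of the player.
; On possessing an enemy character it caches the pawn and runs the behavior tree.
; Perception updates cache the player character when detected, then check whether it was sensed successfully.
; A successful sense sets the blackboard Target and InCombat state, while any other update clears Target and returns the enemy to Patrol.
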(event `self.ReceivePossess`
  (params (PossessedPawn :type "Pawn Object Reference"))
  (bind _asmy_enemy_character (cast `MyEnemyCharacter` PossessedPawn))
  (set `self.EnemyCharacter` _asmy_enemy_character)
  (`self.RunBehaviorTree` (`self.BehaviorTree`)))

(event `self.ReceiveTick`
  (params (DeltaSeconds :type "Float (single-precision)")))

(event `self.PerceptionComponent.OnTargetPerceptionUpdated`
  (params (Actor :type "Actor Object Reference") (Stimulus :type "AIStimulus Structure"))
  (bind _asmy_player_character (cast `MyPlayerCharacter` Actor))
  (set `self.PlayerCharacter` _asmy_player_character))

(event `self.PerceptionComponent.OnTargetPerceptionInfoUpdated`
  (params (UpdateInfo :type "ActorPerceptionUpdateInfo Structure (by ref)"))
  (bind (_targetid _target _stimulus) (break `ActorPerceptionUpdateInfo` UpdateInfo))
  (bind _enemycharacter (`self.EnemyCharacter`))
  (bind _output_get (set `self.SeeingPlayer` (and (== (`self.PlayerCharacter`) _target) (`.bSuccessfullySensed` (break `AIStimulus` _stimulus)))))
  (if _output_get
    (bind _output_get_2 (set `self.SeenActor` _target))
    (`BlackboardComponent.SetValueAsObject` (`self.Blackboard`) (`KismetStringLibrary.Conv_StringToName` "Target") _output_get_2)
    (set `MyBaseCharacter.CurrentState` "InCombat" _enemycharacter)
    (else
      (set `self.SeenActor` null)
      (`BlackboardComponent.SetValueAsObject` (`self.Blackboard`) (`KismetStringLibrary.Conv_StringToName` "Target") null)
      (set `MyBaseCharacter.CurrentState` "Patrol" _enemycharacter))))

(fn `UserConstructionScript`)